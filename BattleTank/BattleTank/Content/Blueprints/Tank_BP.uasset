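; Player-controllable tank Blueprint that wires aiming, track movement, camera and a health bar.
; On BeginPlay it hands its turret, barrel and tracks to the TankAiming and TankMovement components and links itself to the health bar widget.
; Input axes rotate the azimuth gimbal and spring arm and send move and turn intents to TankMovement.
; Fire calls TankAiming, while holding SwitchCam toggles between the two cameras.
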(event `self.ReceiveBeginPlay`
  (`TankAimingComponent.Initialize` (`self.TankAiming`) (`self.TTurretCustom`) (`self.TBarrelCustom`))
  (`TankMovementComponent.Initialize` (`self.TankMovement`) (`self.TLeftTrack`) (`self.TRightTrack`))
  (`self.Initialize Health Bar Widget`))

(event `InputAxis|AimAzimuth`
  (params (AxisValue :type "Float (single-precision)"))
  ;[1 1 1] Ballistics binding
  (`SceneComponent.K2_AddLocalRotation` (`self.Azimuth Gimbal`) (`KismetMathLibrary.MakeRotator` 0.0 0.0 (* AxisValue (`GameplayStatics.GetWorldDeltaSeconds`) 100.0)) false false))

(event `InputAxis|AimElevation`
  (params (AxisValue :type "Float (single-precision)"))
  ;[1 1 1] Ballistics binding
  (`SceneComponent.K2_AddLocalRotation` (`self.SpringArm`) (`KismetMathLibrary.MakeRotator` 0.0 (* AxisValue (`GameplayStatics.GetWorldDeltaSeconds`) 100.0)) false false))

(event `InputAction|Fire`
  (params (Key :type "Key Structure"))
  ;[1 1 1] Ballistics binding
  (:`Pressed`
    (`TankAimingComponent.Fire` (`self.TankAiming`))))

(event `InputAxis|LeftStickForwardBackward`
  (params (AxisValue :type "Float (single-precision)"))
  ;[1 1 1] Movement input binding
  (`TankMovementComponent.IntendMoveForward` (`self.TankMovement`) AxisValue))

(event `InputAxis|LeftStickLeftRight`
  (params (AxisValue :type "Float (single-precision)"))
  ;[1 1 1] Movement input binding
  (`TankMovementComponent.IntendTurnRight` (`self.TankMovement`) AxisValue))

(event `InputAction|SwitchCam`
  (params (Key :type "Key Structure"))
  (:`Pressed`
    (`ActorComponent.ToggleActive` (`self.FPCamera`))
    (`ActorComponent.ToggleActive` (`self.Camera`)))
  (:`Released`
    (`ActorComponent.ToggleActive` (`self.Camera`))
    (`ActorComponent.ToggleActive` (`self.FPCamera`))))

(fn `Initialize Health Bar Widget`
  (bind _ashealth_bar (cast `/Game/Blueprints/HealthBar` (`WidgetComponent.GetUserWidgetObject` (`self.Widget`)))
    (:`then`
      (set `/Game/Blueprints/HealthBar.Tank` self _ashealth_bar))
    (:`CastFailed`
      (`KismetSystemLibrary.PrintString` "ERROR: Health Bar cast Failed")))
  (return))

(fn `UserConstructionScript`)